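; BP_GhostPrototype is a prototype ghost enemy that hunts the player and ends the game on contact.
; Pawn sensing starts a chase via AI MoveTo, slowed inside a cross's overlap, more so for demons.
; Overlapping an unused sage skips the chase and rewrites the blackboard wander Range, which BeginPlay also sets.
; Hitting an unhidden, killable player shows Game Over, pauses the game and destroys the player.
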(event `self.PawnSensing.OnSeePawn`
  (params (Pawn :type "Pawn Object Reference"))
  ;[1 1 1] Ghost hunt logic
  (bind _asbp_first_person_character (cast `/Game/FirstPerson/Blueprints/BP_FirstPersonCharacter` Pawn))
  (bind _returnvalue (`GameplayStatics.GetActorOfClass` "/Game/MY_Blueprints/BP_Sage.BP_Sage_C"))
  (if (`self.IsOverlappingActor` _returnvalue)
    (if (`/Game/MY_Blueprints/BP_Sage.Used` _returnvalue)
      (bind _returnvalue_2 (`GameplayStatics.GetActorOfClass` "/Game/MY_Blueprints/BP_Cross.BP_Cross_C" :!label _label))
      (bind _asbp_cross (cast `/Game/MY_Blueprints/BP_Cross` _returnvalue_2))
      (if (`self.IsOverlappingActor` _asbp_cross)
        (if (`/Game/FirstPerson/Blueprints/BP_FirstPersonCharacter.GhostIsDemon` _asbp_first_person_character)
          (set `CharacterMovementComponent.MaxWalkSpeed` 150.0 (`self.CharacterMovement`))
          (`|AIMoveTo` self (0.0 0.0 0.0) _asbp_first_person_character
            (:`then`
              (`KismetSystemLibrary.Delay` 1.0)))
          (else
            (set `CharacterMovementComponent.MaxWalkSpeed` 250.0 (`self.CharacterMovement`))
            (`|AIMoveTo` self (0.0 0.0 0.0) _asbp_first_person_character
              (:`then`
                (`KismetSystemLibrary.Delay` 1.0)))))
        (else
          (set `CharacterMovementComponent.MaxWalkSpeed` 500.0 (`self.CharacterMovement`))
          (`|AIMoveTo` self (0.0 0.0 0.0) _asbp_first_person_character
            (:`then`
              (`KismetSystemLibrary.Delay` 1.0)))))
      (else
        (`BlackboardComponent.SetValueAsFloat` (`AIBlueprintHelperLibrary.GetBlackboard` null) "Range" (`self.Range`))))
    (else
      (goto _label))))

(event `self.ReceiveBeginPlay`
  ;[1 1 1] set ghost random movement
  (`BlackboardComponent.SetValueAsFloat` (`AIBlueprintHelperLibrary.GetBlackboard` null) "Range" (`self.Range`)))

(event `self.ReceiveHit`
  (params (MyComp :type "PrimitiveComponent Object Reference") (Other :type "Actor Object Reference") (OtherComp :type "PrimitiveComponent Object Reference") (bSelfMoved :type Boolean) (HitLocation :type "Vector Structure") (HitNormal :type "Vector Structure") (NormalImpulse :type "Vector Structure") (Hit :type "HitResult Structure (by ref)"))
  (bind _returnvalue (`GameplayStatics.GetPlayerCharacter` 0))
  (bind _returnvalue_2 (`GameplayStatics.GetPlayerCharacter` 0))
  (bind _returnvalue_3 (`PlayerState.GetPlayerController` (`Pawn.PlayerState` _returnvalue)))
  ;[1 1 1] Kill player/end game
  (if (== Other _returnvalue_2)
    (bind _asbp_first_person_character (cast `/Game/FirstPerson/Blueprints/BP_FirstPersonCharacter` _returnvalue_2))
    (if (`/Game/FirstPerson/Blueprints/BP_FirstPersonCharacter.IsHiding` _asbp_first_person_character)
      _
      (elif (`/Game/FirstPerson/Blueprints/BP_FirstPersonCharacter.can be killed` _asbp_first_person_character)
        (`GameplayStatics.PlaySound2D` "/Game/Sounds/male_02_death_emote_24_Cue.male_02_death_emote_24_Cue" 1.0 1.0 0.0 null null)
        (bind _returnvalue_4 (`|CreateWidget` "/Game/MY_Blueprints/UI/GameOver.GameOver_C" _returnvalue_3))
        (`UserWidget.AddToViewport` _returnvalue_4 0)
        (set `PlayerController.bShowMouseCursor` true _returnvalue_3)
        (`GameplayStatics.SetGamePaused` true)
        (`self.K2_DestroyActor` _returnvalue)
        (`GameplayStatics.PlaySound2D` "/Game/Sounds/Bloody_Nightmare_-_Horror_Impacts_-_Wind_From_Hell_Cue.Bloody_Nightmare_-_Horror_Impacts_-_Wind_From_Hell_Cue" 1.0 1.0 0.0 null null)))))

(fn `UserConstructionScript`)