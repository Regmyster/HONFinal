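; Tutorial prototype ghost enemy that hunts the first-person player when PawnSensing spots them.
; A sighting triggers AIMoveTo toward the player at reduced speed while overlapping BP_Cross, unless the ghost overlaps an unused BP_Sage.
; In that sage case it only writes Range to the blackboard, as BeginPlay does for random movement.
; The kill and game-over logic, which spares hiding players, is disconnected from the empty Hit event.
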(event `self.PawnSensing.OnSeePawn`
  (params (Pawn :type "Pawn Object Reference"))
  ;[1 1 1] Ghost hunt logic
  (bind _asbp_first_person_character (cast `/Game/FirstPerson/Blueprints/BP_FirstPersonCharacter` Pawn))
  (bind _returnvalue (`GameplayStatics.GetActorOfClass` "/Game/MY_Blueprints/BP_Sage.BP_Sage_C"))
  (if (`self.IsOverlappingActor` _returnvalue)
    (if (`/Game/MY_Blueprints/BP_Sage.Used` _returnvalue)
      (bind _returnvalue_2 (`GameplayStatics.GetActorOfClass` "/Game/MY_Blueprints/BP_Cross.BP_Cross_C" :!label _label))
      (bind _asbp_cross (cast `/Game/MY_Blueprints/BP_Cross` _returnvalue_2))
      (if (`self.IsOverlappingActor` _asbp_cross)
        (set `CharacterMovementComponent.MaxWalkSpeed` 250.0 (`self.CharacterMovement`))
        (`|AIMoveTo` self (0.0 0.0 0.0) _asbp_first_person_character
          (:`then`
            (`KismetSystemLibrary.Delay` 1.0)))
        (else
          (set `CharacterMovementComponent.MaxWalkSpeed` 500.0 (`self.CharacterMovement`))
          (`|AIMoveTo` self (0.0 0.0 0.0) _asbp_first_person_character
            (:`then`
              (`KismetSystemLibrary.Delay` 1.0)))))
      (else
        (`BlackboardComponent.SetValueAsFloat` (`AIBlueprintHelperLibrary.GetBlackboard` null) "Range" (`self.Range`))))
    (else
      (goto _label))))

(event `self.ReceiveBeginPlay`
  ;[1 1 1] set ghost random movement
  (`BlackboardComponent.SetValueAsFloat` (`AIBlueprintHelperLibrary.GetBlackboard` null) "Range" (`self.Range`)))

(event `self.ReceiveHit`
  (params (MyComp :type "PrimitiveComponent Object Reference") (Other :type "Actor Object Reference") (OtherComp :type "PrimitiveComponent Object Reference") (bSelfMoved :type Boolean) (HitLocation :type "Vector Structure") (HitNormal :type "Vector Structure") (NormalImpulse :type "Vector Structure") (Hit :type "HitResult Structure (by ref)"))
  ;[1 1 1] Kill player/end game
)

(fn `UserConstructionScript`)