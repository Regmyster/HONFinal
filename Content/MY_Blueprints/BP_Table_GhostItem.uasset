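; Haunted table item that reacts to ghost actions and feeds the player's EMF reader.
; GhostActionOccur rotates the table's TestBox and plays TableMoved.
; Three EMF level volumes set matching flags on BP_EMF when the player enters with EMF active while the item is Active, and clear them on exit regardless of Active.
; IsStrigoi disables all EMF responses; player and reader are found via GetActorOfClass.
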(event `self.EMF Level 1.OnComponentBeginOverlap`
  (params (OverlappedComponent :type "PrimitiveComponent Object Reference") (OtherActor :type "Actor Object Reference") (OtherComp :type "PrimitiveComponent Object Reference") (OtherBodyIndex :type Integer) (bFromSweep :type Boolean) (SweepResult :type "HitResult Structure (by ref)"))
  (if (`self.IsStrigoi`)
    _
    (elif (`self.Active`)
      (bind _returnvalue (`GameplayStatics.GetActorOfClass` "/Game/FirstPerson/Blueprints/BP_FirstPersonCharacter.BP_FirstPersonCharacter_C"))
      (if (== OtherActor _returnvalue)
        (if (`/Game/FirstPerson/Blueprints/BP_FirstPersonCharacter.EMFActive` _returnvalue)
          (bind _returnvalue_2 (`GameplayStatics.GetActorOfClass` "/Game/MY_Blueprints/BP_EMF.BP_EMF_C"))
          (set `/Game/MY_Blueprints/BP_EMF.EMF1` true _returnvalue_2))))))

(event `self.EMF Level 1.OnComponentEndOverlap`
  (params (OverlappedComponent :type "PrimitiveComponent Object Reference") (OtherActor :type "Actor Object Reference") (OtherComp :type "PrimitiveComponent Object Reference") (OtherBodyIndex :type Integer))
  (if (not (`self.IsStrigoi`))
    (if (`self.Active`)
      _
      (else
        _))
    (bind _returnvalue (`GameplayStatics.GetActorOfClass` "/Game/FirstPerson/Blueprints/BP_FirstPersonCharacter.BP_FirstPersonCharacter_C"))
    (if (== OtherActor _returnvalue)
      (if (`/Game/FirstPerson/Blueprints/BP_FirstPersonCharacter.EMFActive` _returnvalue)
        (bind _returnvalue_2 (`GameplayStatics.GetActorOfClass` "/Game/MY_Blueprints/BP_EMF.BP_EMF_C"))
        (set `/Game/MY_Blueprints/BP_EMF.EMF1` false _returnvalue_2)))))

(event `self.EMF Level 2.OnComponentBeginOverlap`
  (params (OverlappedComponent :type "PrimitiveComponent Object Reference") (OtherActor :type "Actor Object Reference") (OtherComp :type "PrimitiveComponent Object Reference") (OtherBodyIndex :type Integer) (bFromSweep :type Boolean) (SweepResult :type "HitResult Structure (by ref)"))
  (if (`self.IsStrigoi`)
    _
    (elif (`self.Active`)
      (bind _returnvalue (`GameplayStatics.GetActorOfClass` "/Game/FirstPerson/Blueprints/BP_FirstPersonCharacter.BP_FirstPersonCharacter_C"))
      (if (== OtherActor _returnvalue)
        (if (`/Game/FirstPerson/Blueprints/BP_FirstPersonCharacter.EMFActive` _returnvalue)
          (bind _returnvalue_2 (`GameplayStatics.GetActorOfClass` "/Game/MY_Blueprints/BP_EMF.BP_EMF_C"))
          (set `/Game/MY_Blueprints/BP_EMF.EMF2` true _returnvalue_2))))))

(event `self.EMF Level 2.OnComponentEndOverlap`
  (params (OverlappedComponent :type "PrimitiveComponent Object Reference") (OtherActor :type "Actor Object Reference") (OtherComp :type "PrimitiveComponent Object Reference") (OtherBodyIndex :type Integer))
  (if (not (`self.IsStrigoi`))
    (if (`self.Active`)
      _
      (else
        _))
    (bind _returnvalue (`GameplayStatics.GetActorOfClass` "/Game/FirstPerson/Blueprints/BP_FirstPersonCharacter.BP_FirstPersonCharacter_C"))
    (if (== OtherActor _returnvalue)
      (if (`/Game/FirstPerson/Blueprints/BP_FirstPersonCharacter.EMFActive` _returnvalue)
        (bind _returnvalue_2 (`GameplayStatics.GetActorOfClass` "/Game/MY_Blueprints/BP_EMF.BP_EMF_C"))
        (set `/Game/MY_Blueprints/BP_EMF.EMF2` false _returnvalue_2)))))

(event `self.EMF Level 3.OnComponentBeginOverlap`
  (params (OverlappedComponent :type "PrimitiveComponent Object Reference") (OtherActor :type "Actor Object Reference") (OtherComp :type "PrimitiveComponent Object Reference") (OtherBodyIndex :type Integer) (bFromSweep :type Boolean) (SweepResult :type "HitResult Structure (by ref)"))
  (if (`self.IsStrigoi`)
    _
    (elif (`self.Active`)
      (bind _returnvalue (`GameplayStatics.GetActorOfClass` "/Game/FirstPerson/Blueprints/BP_FirstPersonCharacter.BP_FirstPersonCharacter_C"))
      (if (== OtherActor _returnvalue)
        (if (`/Game/FirstPerson/Blueprints/BP_FirstPersonCharacter.EMFActive` _returnvalue)
          (bind _returnvalue_2 (`GameplayStatics.GetActorOfClass` "/Game/MY_Blueprints/BP_EMF.BP_EMF_C"))
          (set `/Game/MY_Blueprints/BP_EMF.EMF3` true _returnvalue_2))))))

(event `self.EMF Level 3.OnComponentEndOverlap`
  (params (OverlappedComponent :type "PrimitiveComponent Object Reference") (OtherActor :type "Actor Object Reference") (OtherComp :type "PrimitiveComponent Object Reference") (OtherBodyIndex :type Integer))
  (if (not (`self.IsStrigoi`))
    (if (`self.Active`)
      _
      (else
        _))
    (bind _returnvalue (`GameplayStatics.GetActorOfClass` "/Game/FirstPerson/Blueprints/BP_FirstPersonCharacter.BP_FirstPersonCharacter_C"))
    (if (== OtherActor _returnvalue)
      (if (`/Game/FirstPerson/Blueprints/BP_FirstPersonCharacter.EMFActive` _returnvalue)
        (bind _returnvalue_2 (`GameplayStatics.GetActorOfClass` "/Game/MY_Blueprints/BP_EMF.BP_EMF_C"))
        (set `/Game/MY_Blueprints/BP_EMF.EMF3` false _returnvalue_2)))))

(event `self.GhostActionOccur`
  (`SceneComponent.K2_AddLocalRotation` (`self.TestBox`) (struct :`Yaw` 20.0) false false)
  (`AudioComponent.Play` (`self.TableMoved`) 0.0))

(fn `UserConstructionScript`
  (`parent.UserConstructionScript`))