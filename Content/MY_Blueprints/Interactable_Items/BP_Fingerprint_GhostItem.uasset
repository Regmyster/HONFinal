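; BP_Fingerprint_GhostItem is an interactable ghost item that shows a hidden fingerprint when caught in a beam.
; GhostActionOccur arms the fingerprint; afterwards, a Box begin overlap checks overlapping components for the In_Beam tag and makes TestBox visible with physics-only collision.
; Any Box end overlap hides TestBox and disables its collision.
; An older InLight check on the first-person character remains as unconnected logic.
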(event `self.ReceiveActorBeginOverlap`
  (params (OtherActor :type "Actor Object Reference")))

(event `self.Box.OnComponentBeginOverlap`
  (params (OverlappedComponent :type "PrimitiveComponent Object Reference") (OtherActor :type "Actor Object Reference") (OtherComp :type "PrimitiveComponent Object Reference") (OtherBodyIndex :type Integer) (bFromSweep :type Boolean) (SweepResult :type "HitResult Structure (by ref)"))
  (if (`self.FingerprintActive`)
    (for _array_element (`PrimitiveComponent.GetOverlappingComponents` OverlappedComponent)
      (if (`ActorComponent.ComponentHasTag` _array_element "In_Beam")
        (`SceneComponent.SetVisibility` (`self.TestBox`) true false)
        (`PrimitiveComponent.SetCollisionEnabled` (`self.TestBox`) "PhysicsOnly")
        (break)))))

(event `self.Box.OnComponentEndOverlap`
  (params (OverlappedComponent :type "PrimitiveComponent Object Reference") (OtherActor :type "Actor Object Reference") (OtherComp :type "PrimitiveComponent Object Reference") (OtherBodyIndex :type Integer))
  (`SceneComponent.SetVisibility` (`self.TestBox`) false false)
  (`PrimitiveComponent.SetCollisionEnabled` (`self.TestBox`) "NoCollision"))

(event `self.GhostActionOccur`
  (set `self.FingerprintActive` true))

(fn `UserConstructionScript`
  (`parent.UserConstructionScript`))