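; BP_GhostItem is an interactable item that gives EMF readings while a ghost action is happening.
; GhostActionOccur and GhostActionEnd toggle an Active flag that gates three overlap components, EMFLevel1 to EMFLevel3.
; While active, beginning an overlap sets the matching level flag on the BP_EMF found via GetActorOfClass.
; Ending an overlap clears that flag regardless of Active, and neither overlap event checks which actor is overlapping.
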(event `GhostActionEnd`
  (set `self.Active` false))

(event `GhostActionOccur`
  (set `self.Active` true))

(event `self.EMF Level 1.OnComponentBeginOverlap`
  (params (OverlappedComponent :type "PrimitiveComponent Object Reference") (OtherActor :type "Actor Object Reference") (OtherComp :type "PrimitiveComponent Object Reference") (OtherBodyIndex :type Integer) (bFromSweep :type Boolean) (SweepResult :type "HitResult Structure (by ref)"))
  (if (`self.Active`)
    (bind _returnvalue (`GameplayStatics.GetActorOfClass` "/Game/MY_Blueprints/BP_EMF.BP_EMF_C"))
    (set `/Game/MY_Blueprints/BP_EMF.EMF1` true _returnvalue)))

(event `self.EMF Level 1.OnComponentEndOverlap`
  (params (OverlappedComponent :type "PrimitiveComponent Object Reference") (OtherActor :type "Actor Object Reference") (OtherComp :type "PrimitiveComponent Object Reference") (OtherBodyIndex :type Integer))
  (bind _returnvalue (`GameplayStatics.GetActorOfClass` "/Game/MY_Blueprints/BP_EMF.BP_EMF_C"))
  (set `/Game/MY_Blueprints/BP_EMF.EMF1` false _returnvalue))

(event `self.EMF Level 2.OnComponentBeginOverlap`
  (params (OverlappedComponent :type "PrimitiveComponent Object Reference") (OtherActor :type "Actor Object Reference") (OtherComp :type "PrimitiveComponent Object Reference") (OtherBodyIndex :type Integer) (bFromSweep :type Boolean) (SweepResult :type "HitResult Structure (by ref)"))
  (if (`self.Active`)
    (bind _returnvalue (`GameplayStatics.GetActorOfClass` "/Game/MY_Blueprints/BP_EMF.BP_EMF_C"))
    (set `/Game/MY_Blueprints/BP_EMF.EMF2` true _returnvalue)))

(event `self.EMF Level 2.OnComponentEndOverlap`
  (params (OverlappedComponent :type "PrimitiveComponent Object Reference") (OtherActor :type "Actor Object Reference") (OtherComp :type "PrimitiveComponent Object Reference") (OtherBodyIndex :type Integer))
  (bind _returnvalue (`GameplayStatics.GetActorOfClass` "/Game/MY_Blueprints/BP_EMF.BP_EMF_C"))
  (set `/Game/MY_Blueprints/BP_EMF.EMF2` false _returnvalue))

(event `self.EMF Level 3.OnComponentBeginOverlap`
  (params (OverlappedComponent :type "PrimitiveComponent Object Reference") (OtherActor :type "Actor Object Reference") (OtherComp :type "PrimitiveComponent Object Reference") (OtherBodyIndex :type Integer) (bFromSweep :type Boolean) (SweepResult :type "HitResult Structure (by ref)"))
  (if (`self.Active`)
    (bind _returnvalue (`GameplayStatics.GetActorOfClass` "/Game/MY_Blueprints/BP_EMF.BP_EMF_C"))
    (set `/Game/MY_Blueprints/BP_EMF.EMF3` true _returnvalue)))

(event `self.EMF Level 3.OnComponentEndOverlap`
  (params (OverlappedComponent :type "PrimitiveComponent Object Reference") (OtherActor :type "Actor Object Reference") (OtherComp :type "PrimitiveComponent Object Reference") (OtherBodyIndex :type Integer))
  (bind _returnvalue (`GameplayStatics.GetActorOfClass` "/Game/MY_Blueprints/BP_EMF.BP_EMF_C"))
  (set `/Game/MY_Blueprints/BP_EMF.EMF3` false _returnvalue))

(fn `UserConstructionScript`)