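; Hiding spot Blueprint that lets the first-person character toggle hiding with the Hide input while overlapping its Box.
; The overlap enables actor input and opens a gate; leaving disables both.
; Hiding calls the character's Hide and blends the view to this actor, where a self-repeating short-delay loop applies clamped mouse pitch and yaw to its Camera.
; When not hiding, mouse look passes through to the character.
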(event `InputAction|Hide`
  (params (Key :type "Key Structure"))
  (bind _as_bp_first_person_character (`self.As BP First Person Character`))
  (:`Pressed`
    (`/Engine/EditorBlueprintResources/StandardMacros.Gate` true :!label _label
      (:`Exit`
        (if (`/Game/FirstPerson/Blueprints/BP_FirstPersonCharacter.IsHiding` _as_bp_first_person_character)
          (`/Game/FirstPerson/Blueprints/BP_FirstPersonCharacter.Unhide` _as_bp_first_person_character)
          (else
            (`/Game/FirstPerson/Blueprints/BP_FirstPersonCharacter.Hide` _as_bp_first_person_character)
            (`|ExecutionSequence`
              (:`then_0`
                (`PlayerController.SetViewTargetWithBlend` (`GameplayStatics.GetPlayerController` 0) self 0.5 "VTBlend_Linear" 0.0 false)
                (`self.MoveCamera`))
              (:`then_1`
                (`KismetSystemLibrary.Delay` 0.2)
                (`self.EnableInput` (`GameplayStatics.GetPlayerController` 0) :!label _label_2)
                (goto _label :!via `Open`)))))))))

(event `self.Box.OnComponentBeginOverlap`
  (params (OverlappedComponent :type "PrimitiveComponent Object Reference") (OtherActor :type "Actor Object Reference") (OtherComp :type "PrimitiveComponent Object Reference") (OtherBodyIndex :type Integer) (bFromSweep :type Boolean) (SweepResult :type "HitResult Structure (by ref)"))
  (bind _asbp_first_person_character (cast `/Game/FirstPerson/Blueprints/BP_FirstPersonCharacter` OtherActor))
  (set `self.As BP First Person Character` _asbp_first_person_character)
  (goto _label_2))

(event `self.Box.OnComponentEndOverlap`
  (params (OverlappedComponent :type "PrimitiveComponent Object Reference") (OtherActor :type "Actor Object Reference") (OtherComp :type "PrimitiveComponent Object Reference") (OtherBodyIndex :type Integer))
  (cast `/Game/FirstPerson/Blueprints/BP_FirstPersonCharacter` OtherActor)
  (`self.DisableInput` (`GameplayStatics.GetPlayerController` 0))
  (goto _label :!via `Close`))

(event `MoveCamera`
  (if (`/Game/FirstPerson/Blueprints/BP_FirstPersonCharacter.IsHiding` (`self.As BP First Person Character`))
    (`SceneComponent.K2_SetRelativeRotation` (`self.Camera`) (`KismetMathLibrary.MakeRotator` 0.0 (`KismetMathLibrary.FClamp` (* (stale `InputAxis|Look Up / Down Mouse` _output_get) -1.0) -10.0 10.0) (`KismetMathLibrary.FClamp` (stale `InputAxis|Turn Right / Left Mouse` _output_get) 20.0 150.0)) false false)
    (`KismetSystemLibrary.Delay` 0.001)
    (`self.MoveCamera`)))

(event `InputAxis|Look Up / Down Mouse`
  (params (AxisValue :type "Float (single-precision)"))
  (bind _as_bp_first_person_character (`self.As BP First Person Character`))
  (if (`/Game/FirstPerson/Blueprints/BP_FirstPersonCharacter.IsHiding` _as_bp_first_person_character)
    (bind _output_get (set `self.Pitch` (+ (`self.Pitch`) AxisValue)))
    (else
      (`Pawn.AddControllerPitchInput` _as_bp_first_person_character AxisValue))))

(event `InputAxis|Turn Right / Left Mouse`
  (params (AxisValue :type "Float (single-precision)"))
  (bind _as_bp_first_person_character (`self.As BP First Person Character`))
  (if (`/Game/FirstPerson/Blueprints/BP_FirstPersonCharacter.IsHiding` _as_bp_first_person_character)
    (bind _output_get (set `self.Yaw` (+ (`self.Yaw`) AxisValue)))
    (else
      (`Pawn.AddControllerYawInput` _as_bp_first_person_character AxisValue))))

(fn `UserConstructionScript`)