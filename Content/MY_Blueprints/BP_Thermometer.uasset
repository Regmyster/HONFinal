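; BP_Thermometer is a thermometer actor that switches between normal and cold states as it overlaps volumes tagged "coldroom".
; On begin overlap it checks whether it overlaps the first ColdRoomTUto in the level, latching RightGhost, which is never reset here.
; Once RightGhost is set, entering any tagged volume sets ItCold and clears ItNormal.
; Leaving a tagged volume restores the normal state.
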(event `self.ReceiveActorEndOverlap`
  (params (OtherActor :type "Actor Object Reference"))
  (if (`self.ActorHasTag` OtherActor "coldroom")
    (set `self.itNormal` true)
    (set `self.itCold` false)))

(event `self.ReceiveActorBeginOverlap`
  (params (OtherActor :type "Actor Object Reference"))
  (if (`self.ActorHasTag` OtherActor "coldroom")
    (bind _outactors (`GameplayStatics.GetAllActorsOfClass` "/Game/MY_Blueprints/ColdRoomTUto.ColdRoomTUto_C"))
    (if (`self.IsOverlappingActor` (`|GetArrayItem` _outactors))
      (set `self.RightGhost` true))
    (if (`self.RightGhost`)
      (set `self.itNormal` false)
      (set `self.itCold` true))))

(event `self.ReceiveTick`
  (params (DeltaSeconds :type "Float (single-precision)")))

(fn `UserConstructionScript`)