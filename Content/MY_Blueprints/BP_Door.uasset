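; BP_Door is an interactable door that swings open and closed by rotating its DoorSM mesh in yaw.
; Interact checks IsOpen, sets the OpenDoorT timeline's play rate from TimeToOpen or TimeToClose, then plays or reverses it.
; The timeline's DoorTrack lerps yaw between the closed and open values, and IsOpen toggles when the timeline finishes.
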(event `OpenDoor`
  (bind (_direction _door_track) (`Timeline|Open Door T` :!label _label)
    (:`Update`
      (`SceneComponent.K2_SetRelativeRotation` (`self.Door SM`) (`KismetMathLibrary.MakeRotator` 0.0 0.0 (`KismetMathLibrary.Lerp` (`self.ClosePostition`) (`self.OpenPostition`) _door_track)) false false))
    (:`Finished`
      (set `self.IsOpen` (not (`self.IsOpen`))))))

(event `CloseDoor`
  (goto _label :!via `Reverse`))

(fn `Interact`
  (params (Interactor :type "Character Object Reference"))
  (returns (`Did Interact?` :type Boolean))
  (if (not (`self.IsOpen`))
    (`TimelineComponent.SetPlayRate` (`self.Open Door T`) (/ 1.0 (`self.TimeToOpen`)))
    (`self.OpenDoor`)
    (else
      (`TimelineComponent.SetPlayRate` (`self.Open Door T`) (/ 1.0 (`self.TimeToClose`)))
      (`self.CloseDoor`)))
  (return true))

(fn `UserConstructionScript`)