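; BP_Fingerprint is a fingerprint actor that shows or hides its FPBox depending on light.
; When the first-person character overlaps the actor, its InLight flag toggles FPBox visibility and switches collision between PhysicsOnly and none.
; Box begin overlap also reveals FPBox if any component overlapping the triggering component is tagged In_Beam.
; Any Box end overlap hides it and disables collision, without checking for remaining beam overlaps.
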(event `self.ReceiveActorBeginOverlap`
  (params (OtherActor :type "Actor Object Reference"))
  (bind _asbp_first_person_character (cast `/Game/FirstPerson/Blueprints/BP_FirstPersonCharacter` OtherActor))
  (if (`/Game/FirstPerson/Blueprints/BP_FirstPersonCharacter.In_Light` _asbp_first_person_character)
    (`SceneComponent.SetVisibility` (`self.FPBox`) true false)
    (`PrimitiveComponent.SetCollisionEnabled` (`self.FPBox`) "PhysicsOnly")
    (else
      (`SceneComponent.SetVisibility` (`self.FPBox`) false false)
      (`PrimitiveComponent.SetCollisionEnabled` (`self.FPBox`) "NoCollision"))))

(event `self.Box.OnComponentBeginOverlap`
  (params (OverlappedComponent :type "PrimitiveComponent Object Reference") (OtherActor :type "Actor Object Reference") (OtherComp :type "PrimitiveComponent Object Reference") (OtherBodyIndex :type Integer) (bFromSweep :type Boolean) (SweepResult :type "HitResult Structure (by ref)"))
  (for _array_element (`PrimitiveComponent.GetOverlappingComponents` OverlappedComponent)
    (if (`ActorComponent.ComponentHasTag` _array_element "In_Beam")
      (`SceneComponent.SetVisibility` (`self.FPBox`) true false)
      (`PrimitiveComponent.SetCollisionEnabled` (`self.FPBox`) "PhysicsOnly")
      (break))))

(event `self.Box.OnComponentEndOverlap`
  (params (OverlappedComponent :type "PrimitiveComponent Object Reference") (OtherActor :type "Actor Object Reference") (OtherComp :type "PrimitiveComponent Object Reference") (OtherBodyIndex :type Integer))
  (`SceneComponent.SetVisibility` (`self.FPBox`) false false)
  (`PrimitiveComponent.SetCollisionEnabled` (`self.FPBox`) "NoCollision"))

(fn `UserConstructionScript`)