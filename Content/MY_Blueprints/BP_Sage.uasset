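; BP_Sage is a single-use sage item that resets the ghost when lit with Q.
; Player overlap with the InHand component toggles input for the item.
; Lighting plays a sound, enables Sphere collision, then destroys and respawns both regular and tutorial ghost classes at their current transforms.
; After five seconds it marks itself used and disables the Sphere, which also starts disabled.
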(event `self.inHand.OnComponentBeginOverlap`
  (params (OverlappedComponent :type "PrimitiveComponent Object Reference") (OtherActor :type "Actor Object Reference") (OtherComp :type "PrimitiveComponent Object Reference") (OtherBodyIndex :type Integer) (bFromSweep :type Boolean) (SweepResult :type "HitResult Structure (by ref)"))
  ;[1 1 1] enable keyboard use when in hand
  (cast `/Game/FirstPerson/Blueprints/BP_FirstPersonCharacter` OtherActor)
  (`self.EnableInput` (`GameplayStatics.GetPlayerController` 0)))

(event `self.inHand.OnComponentEndOverlap`
  (params (OverlappedComponent :type "PrimitiveComponent Object Reference") (OtherActor :type "Actor Object Reference") (OtherComp :type "PrimitiveComponent Object Reference") (OtherBodyIndex :type Integer))
  ;[1 1 1] enable keyboard use when in hand
  (cast `/Game/FirstPerson/Blueprints/BP_FirstPersonCharacter` OtherActor)
  (`self.DisableInput` (`GameplayStatics.GetPlayerController` 0)))

(event `Key|Q`
  (params (Key :type "Key Structure"))
  ;[1 1 1] Use the sage
  (:`Pressed`
    (if (not (`self.Used`))
      (`PrimitiveComponent.SetCollisionEnabled` (`self.Sphere`) "QueryAndPhysics")
      (`GameplayStatics.PlaySound2D` "/Game/Sounds/SageLit_Cue.SageLit_Cue" 1.0 1.0 0.0 null null)
      (`|ExecutionSequence`
        (:`then_0`
          (bind _returnvalue (`GameplayStatics.GetActorOfClass` "/Game/Ghosts/BP_GhostPrototype.BP_GhostPrototype_C"))
          (set `self.ghostTransform` (`self.GetTransform` _returnvalue))
          (`self.K2_DestroyActor` _returnvalue)
          (`|SpawnActorFromClass` "/Game/Ghosts/BP_GhostPrototype.BP_GhostPrototype_C" (`self.ghostTransform`) "Undefined" "OverrideRootScale" null null)
          (`KismetSystemLibrary.Delay` 5.0))
        (:`then_1`
          (bind _returnvalue_2 (`GameplayStatics.GetActorOfClass` "/Game/Ghosts/BP_GhostPrototype_tutorial.BP_GhostPrototype_tutorial_C"))
          (set `self.ghostTransform` (`self.GetTransform` _returnvalue_2))
          (`self.K2_DestroyActor` _returnvalue_2)
          (`|SpawnActorFromClass` "/Game/Ghosts/BP_GhostPrototype_tutorial.BP_GhostPrototype_tutorial_C" (`self.ghostTransform`) "Undefined" "OverrideRootScale" null null)
          (`KismetSystemLibrary.Delay` 5.0)))
      (set `self.Used` true)
      (`PrimitiveComponent.SetCollisionEnabled` (`self.Sphere`) "NoCollision"))))

(event `self.ReceiveBeginPlay`
  ;[1 1 1] start the sage as off
  (`PrimitiveComponent.SetCollisionEnabled` (`self.Sphere`) "NoCollision"))

(fn `UserConstructionScript`)