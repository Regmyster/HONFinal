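; BP_Ghost_Interact is an actor whose lamp flickers when a ghost enters it.
; On begin overlap it casts the other actor to BP_GhostPrototype and ignores anything else.
; A chain of fixed short delays toggles the Lamp component's visibility on and off three times, leaving it hidden at the end.
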(event `self.ReceiveActorBeginOverlap`
  (params (OtherActor :type "Actor Object Reference"))
  (bind _lamp (`self.lamp`))
  (bind _lamp_2 (`self.lamp`))
  (bind _lamp_3 (`self.lamp`))
  (cast `/Game/Ghosts/BP_GhostPrototype` OtherActor)
  (`SceneComponent.SetVisibility` _lamp_2 true false)
  (`KismetSystemLibrary.Delay` 0.2)
  (`SceneComponent.SetVisibility` _lamp_2 false false)
  (`KismetSystemLibrary.Delay` 0.2)
  (`SceneComponent.SetVisibility` _lamp_3 true false)
  (`KismetSystemLibrary.Delay` 0.2)
  (`SceneComponent.SetVisibility` _lamp_3 false false)
  (`KismetSystemLibrary.Delay` 0.2)
  (`SceneComponent.SetVisibility` _lamp true false)
  (`KismetSystemLibrary.Delay` 0.2)
  (`SceneComponent.SetVisibility` _lamp false false)
  (`KismetSystemLibrary.Delay` 0.2))

(fn `UserConstructionScript`)