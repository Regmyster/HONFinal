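; BP_HauntedItem is a haunted object that signals its proximity to the EMF reader, BP_EMF, through three overlap zones, EMFLevel1 to EMFLevel3.
; Entering a zone finds the BP_EMF actor via GetActorOfClass and sets the matching EMF1, EMF2 or EMF3 flag, and leaving clears it.
; The overlapping actor is never checked, so any overlap toggles the flags on that single found reader.
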(event `self.EMF Level 1.OnComponentBeginOverlap`
  (params (OverlappedComponent :type "PrimitiveComponent Object Reference") (OtherActor :type "Actor Object Reference") (OtherComp :type "PrimitiveComponent Object Reference") (OtherBodyIndex :type Integer) (bFromSweep :type Boolean) (SweepResult :type "HitResult Structure (by ref)"))
  (bind _returnvalue (`GameplayStatics.GetActorOfClass` "/Game/MY_Blueprints/BP_EMF.BP_EMF_C"))
  (bind _asemf (cast `/Game/MY_Blueprints/BP_EMF` _returnvalue)
    (:`then`
      (set `/Game/MY_Blueprints/BP_EMF.EMF1` true _asemf))
    (:`CastFailed`
      (`KismetSystemLibrary.PrintString` "Failed"))))

(event `self.EMF Level 1.OnComponentEndOverlap`
  (params (OverlappedComponent :type "PrimitiveComponent Object Reference") (OtherActor :type "Actor Object Reference") (OtherComp :type "PrimitiveComponent Object Reference") (OtherBodyIndex :type Integer))
  (bind _returnvalue (`GameplayStatics.GetActorOfClass` "/Game/MY_Blueprints/BP_EMF.BP_EMF_C"))
  (bind _asemf (cast `/Game/MY_Blueprints/BP_EMF` _returnvalue))
  (set `/Game/MY_Blueprints/BP_EMF.EMF1` false _asemf))

(event `self.EMF Level 2.OnComponentBeginOverlap`
  (params (OverlappedComponent :type "PrimitiveComponent Object Reference") (OtherActor :type "Actor Object Reference") (OtherComp :type "PrimitiveComponent Object Reference") (OtherBodyIndex :type Integer) (bFromSweep :type Boolean) (SweepResult :type "HitResult Structure (by ref)"))
  (bind _returnvalue (`GameplayStatics.GetActorOfClass` "/Game/MY_Blueprints/BP_EMF.BP_EMF_C"))
  (bind _asemf (cast `/Game/MY_Blueprints/BP_EMF` _returnvalue))
  (set `/Game/MY_Blueprints/BP_EMF.EMF2` true _asemf))

(event `self.EMF Level 2.OnComponentEndOverlap`
  (params (OverlappedComponent :type "PrimitiveComponent Object Reference") (OtherActor :type "Actor Object Reference") (OtherComp :type "PrimitiveComponent Object Reference") (OtherBodyIndex :type Integer))
  (bind _returnvalue (`GameplayStatics.GetActorOfClass` "/Game/MY_Blueprints/BP_EMF.BP_EMF_C"))
  (bind _asemf (cast `/Game/MY_Blueprints/BP_EMF` _returnvalue))
  (set `/Game/MY_Blueprints/BP_EMF.EMF2` false _asemf))

(event `self.EMF Level 3.OnComponentBeginOverlap`
  (params (OverlappedComponent :type "PrimitiveComponent Object Reference") (OtherActor :type "Actor Object Reference") (OtherComp :type "PrimitiveComponent Object Reference") (OtherBodyIndex :type Integer) (bFromSweep :type Boolean) (SweepResult :type "HitResult Structure (by ref)"))
  (bind _returnvalue (`GameplayStatics.GetActorOfClass` "/Game/MY_Blueprints/BP_EMF.BP_EMF_C"))
  (bind _asemf (cast `/Game/MY_Blueprints/BP_EMF` _returnvalue))
  (set `/Game/MY_Blueprints/BP_EMF.EMF3` true _asemf))

(event `self.EMF Level 3.OnComponentEndOverlap`
  (params (OverlappedComponent :type "PrimitiveComponent Object Reference") (OtherActor :type "Actor Object Reference") (OtherComp :type "PrimitiveComponent Object Reference") (OtherBodyIndex :type Integer))
  (bind _returnvalue (`GameplayStatics.GetActorOfClass` "/Game/MY_Blueprints/BP_EMF.BP_EMF_C"))
  (bind _asemf (cast `/Game/MY_Blueprints/BP_EMF` _returnvalue))
  (set `/Game/MY_Blueprints/BP_EMF.EMF3` false _asemf))

(fn `UserConstructionScript`)